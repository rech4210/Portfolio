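; Gameplay ability for Skill 1, which plays a kick montage against targets chosen by a targeting strategy.
; On activation it commits, applies a tagged SetByCaller cooldown from the skill data asset, then takes instant mouse target data before gathering targets.
; On montage completion, the authority sends notify events to the player state and boss targets, then ends the ability.
; The Blueprint's damage-effect application is disconnected, noted as moving to C++.
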(event `self.K2_ActivateAbility`
  (bind _returnvalue (`GameplayStatics.GetPlayerState` 0))
  ; Apply CoolTime By Tag GE At Start
  (`self.K2_CommitAbility`)
  (bind _returnvalue_2 (`AbilitySystemBlueprintLibrary.AssignTagSetByCallerMagnitude` (`self.MakeOutgoingGameplayEffectSpec` "/Game/Blueprints/Effect/GE_CoolDown.GE_CoolDown_C") (struct :`TagName` "Data.Cooldown") (`SkillDataAsset.CoolTime` (`self.SkillDataAsset`))))
  (bind _returnvalue_3 (`AbilitySystemBlueprintLibrary.AddGrantedTags` _returnvalue_2 (struct :`GameplayTags` (struct :`(TagName` "Data.Cooldown.Skill1")))))
  (`AbilitySystemComponent.BP_ApplyGameplayEffectSpecToSelf` (`self.GetAbilitySystemComponentFromActorInfo`) _returnvalue_3)
  ; Get Mouse Hit Location
  (bind _returnvalue_4 (`|SpawnActorFromClass` "/Script/SkillModule.SkillTargetActor_Mouse" (`KismetMathLibrary.MakeTransform` (0.0 0.0 0.0)) "AlwaysSpawn" "MultiplyWithRoot" null (struct) (struct) null (struct) false null))
  (bind (_asynctaskproxy _data) (`AbilityTask_WaitTargetData.WaitTargetDataUsingActor` "SkillTarget_1" "Instant" _returnvalue_4)
    (:`ValidData`
      (`self.OnTargetDataReceived` _data)
      ; Get Target / 순서 변경 가능
      (bind _returnvalue_5 (`self.GetTargetActorsByStrategy`))
      (set `self.BP_TargetActor` _returnvalue_5)
      ; Montage Execute AbilityTask
      (bind (_asynctaskproxy_2 _eventtag _eventdata) (`GGwaPlayMontageAndWaitForEvent.PlayMontageAndWaitForEvent` "Skill1Task" "/Game/RamsterZ_FreeAnims_Volume1/AnimationSequence/H2H/H2H_Kick02_Montage.H2H_Kick02_Montage" (struct :`GameplayTags` (struct :`(TagName` "Skill.Skill1"))))
        (:`OnCompleted`
          (`self.OnMontageCompleted` _eventtag _eventdata)
          (`self.K2_HasAuthority`
            (:`True`
              (`AbilitySystemBlueprintLibrary.SendGameplayEventToActor` _returnvalue (struct :`TagName` "GasEvent.Notify") (make `GameplayEventData` (struct :`TagName` "Skill.Skill1") _returnvalue null null null (struct) (struct :`GameplayTags` (struct :`(TagName` "Skill.Skill1"))) (struct :`GameplayTags` (struct :`(TagName` "GasEvent.Notify")))))
              (for _array_element (`self.BP_TargetActor`)
                (bind _asboss_character (cast `BossCharacter` _array_element))
                (`AbilitySystemBlueprintLibrary.SendGameplayEventToActor` _asboss_character (struct :`TagName` "GasEvent.Notify")))
              (`self.K2_EndAbility`))))
        (:`OnInterrupted`
          (`self.OnMontageInterrupted` (struct) :!label _label))
        (:`OnCancelled`
          (goto _label))))
    (:`Cancelled`
      (`self.OnTargetDataCancelled` _data))))

(event `self.K2_OnEndAbility`
  (params (bWasCancelled :type Boolean)))